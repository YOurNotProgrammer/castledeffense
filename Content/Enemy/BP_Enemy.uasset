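; BP_Enemy is an enemy actor with health, a widget health bar and an explosion on death.
; Any capsule hit, with no check on what hit it, subtracts fixed damage, prints debug text and pushes health into WG_EnemyHealthBar.
; Tick polls health; at zero or below it plays an explosion sound, calls DestroyActor, then adds a particle component and sets the Dead flag.
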(event OnComponentBeginOverlap(CapsuleComponent)
  (params (OverlappedComponent :type Primitive%20Component%20Object%20Reference) (OtherActor :type Actor%20Object%20Reference) (OtherComp :type Primitive%20Component%20Object%20Reference) (OtherBodyIndex :type Integer) (bFromSweep :type Boolean) (SweepResult :type Hit%20Result%20Structure%20%28by%20ref%29)))

(event OnComponentHit(CapsuleComponent)
  (params (HitComponent :type Primitive%20Component%20Object%20Reference) (OtherActor :type Actor%20Object%20Reference) (OtherComp :type Primitive%20Component%20Object%20Reference) (NormalImpulse :type Vector :default "0, 0, 0") (Hit :type Hit%20Result%20Structure%20%28by%20ref%29))
  (Development|PrintString "enemyhit")
  (Variables|Default|SetEnemyHealth (- (Variables|Default|GetEnemyHealth) 34.0))
  (CallFunction|UpdateHealthBar)
  (Development|PrintString (Utilities|String|ToString(Float) (Variables|Default|GetEnemyHealth))))

(event EventBeginPlay
  (CallFunction|UpdateHealthBar))

(event EventTick
  (params (DeltaSeconds :type Float%20%28single-precision%29))
  (if (<= (Variables|Default|GetEnemyHealth) 0.0)
    (Audio|PlaySound2D "/Game/StarterContent/Audio/Explosion01.Explosion01" 1e+01 1.0 0.0 0 0)
    (Actor|DestroyActor)
    (AddComponent|AddParticleSystemComponent false)
    (Variables|Default|SetDead? true)
    (else
      (Variables|Default|SetDead? false))))

(fn ConstructionScript)

(fn UpdateHealthBar
  (bind _aswg_enemy_health_bar (Utilities|Casting|CastToWG_EnemyHealthBar (UserInterface|GetUserWidgetObject (Variables|Default|GetHealthBar))))
  (Variables|/Game/Enemy/WG_EnemyHealthBar.WG_EnemyHealthBar_C|SetHealth _aswg_enemy_health_bar (Variables|Default|GetEnemyHealth))
  (return))