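; Enemy spawner that spawns BP_EnemyChild AI pawns at its own location in a timed series.
; Tick watches the Start flag, calls SpawnEnemy when it is set, then clears it.
; SpawnEnemy re-calls itself after a fixed delay, incrementing CurrentAmount until it equals MaxAmount.
; Each call spawns before checking the limit, so a pawn also spawns on the call that reaches it.
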(event Custom|SpawnEnemy
  (AI|SpawnAIFromClass "/Game/Enemy/BP_EnemyChild.BP_EnemyChild_C" 0 (Transformation|GetActorLocation) "0, 0, 0" false 0)
  (if (not (== (Variables|Default|GetMaxAmount) (Variables|Default|GetCurrentAmount)))
    (Variables|Default|SetCurrentAmount (+ (Variables|Default|GetCurrentAmount) 1))
    (Utilities|FlowControl|Delay 3.0)
    (CallFunction|SpawnEnemy)))

(event EventTick
  (params (DeltaSeconds :type Float%20%28single-precision%29))
  (if (Variables|Default|GetStart?)
    (CallFunction|SpawnEnemy)
    (Variables|Default|SetStart? false)))

(fn ConstructionScript)