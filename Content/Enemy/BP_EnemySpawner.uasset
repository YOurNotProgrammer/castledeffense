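; Enemy spawner actor that spawns BP_EnemyChild AI at its own location, starting on BeginPlay.
; SpawnEnemy re-calls itself every 3 seconds, incrementing CurrentAmount until it equals MaxAmount.
; Each call spawns before checking the limit; at the limit, it waits 30 seconds, then finds BP_EnemySpawner_2 and sets its Start flag, chaining to the next spawner.
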(event Custom|SpawnEnemy
  (AI|SpawnAIFromClass "/Game/Enemy/BP_EnemyChild.BP_EnemyChild_C" 0 (Transformation|GetActorLocation) "0, 0, 0" false 0)
  (if (== (Variables|Default|GetMaxAmount) (Variables|Default|GetCurrentAmount))
    (Utilities|FlowControl|Delay 3e+01)
    (bind _returnvalue (Actor|GetActorOfClass "/Game/Enemy/BP_EnemySpawner_2.BP_EnemySpawner_2_C"))
    (Variables|/Game/Enemy/BP_EnemySpawner_2.BP_EnemySpawner_2_C|SetStart? _returnvalue true)
    (else
      (Variables|Default|SetCurrentAmount (+ (Variables|Default|GetCurrentAmount) 1))
      (Utilities|FlowControl|Delay 3.0)
      (CallFunction|SpawnEnemy))))

(event EventBeginPlay
  (CallFunction|SpawnEnemy))

(fn ConstructionScript)