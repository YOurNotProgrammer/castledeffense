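; BP_EnemyChild is an enemy Blueprint that runs at a door and self-destructs.
; On BeginPlay it waits briefly, sets its walk speed and uses AI MoveTo toward the first BP_Door found.
; Success and failure both lead to a delay, an explosion sound, DestroyActor, then an AddParticleSystemComponent call after destruction.
; The parent BeginPlay call is disconnected, and no damage is applied here.
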(event EventBeginPlay
  (Utilities|FlowControl|Delay 0.2)
  (Variables|/Script/Engine.CharacterMovementComponent|SetMaxWalkSpeed (Variables|Character|GetCharacterMovement) 6e+02)
  (bind _outactors (Actor|GetAllActorsOfClass "/Game/LevelPrototyping/Door/BP_Door.BP_Door_C"))
  (AI|AIMoveTo self "0, 0, 0" (Utilities|Array|Get(acopy) _outactors) 5.0 false
    (:OnSuccess
      _)
    (:OnFail
      _))
  (Utilities|FlowControl|Delay 3.0)
  (Audio|PlaySound2D "/Game/StarterContent/Audio/Explosion01.Explosion01" 1e+01 1.0 0.0 0 0)
  (Actor|DestroyActor)
  (AddComponent|AddParticleSystemComponent false))

(event Collision|EventActorBeginOverlap
  (params (OtherActor :type Actor%20Object%20Reference)))

(event EventTick
  (params (DeltaSeconds :type Float%20%28single-precision%29))
  (|CallParentFunction DeltaSeconds) ; 지금 이 노드는 비활성 상태입니다. \n핀을 끌어서 다른 노드를 연결하면 활성화됩니다.
)

(fn ConstructionScript
  (|CallParentFunction))